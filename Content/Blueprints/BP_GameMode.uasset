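; Game mode for local multiplayer that sets up players, a shared menu and character spawning.
; On BeginPlay it gathers PlayerStarts and, for each index matching a numeric PlayerStartTag, creates a local player possessing a BP_InputReceiver spawned at that array index's start.
; DisplayCharacterSelect adds a player's selection panel to the menu and links it to their receiver.
; SpawnPlayer spawns a ThirdPersonCharacter at the receiver's transform and has the player's controller possess it.
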(event EventBeginPlay
  (CallFunction|GetPlayerStartPoints)
  (CallFunction|SpawnInputReceivers)
  (bind _returnvalue (UserInterface|CreateWidget "/Game/Blueprints/UI/WBP_Menu.WBP_Menu_C"))
  (bind _output_get (Variables|Default|SetMenuWidjetRed _returnvalue))
  (UserInterface|Viewport|AddtoViewport _output_get 0))

(fn ConstructionScript)

(fn GetPlayerStartPoints
  (bind _outactors (Actor|GetAllActorsOfClass "/Script/Engine.PlayerStart"))
  (Variables|Default|SetPlayerStartArray _outactors))

(fn SpawnInputReceivers
  (for (_ _array_index) (Variables|Default|GetPlayerStartArray)
    (LocalVariables|SetIndex _array_index)
    (for _array_element (Variables|Default|GetPlayerStartArray)
      (if (== (CallFunction|NametoInt _array_element) (LocalVariables|GetIndex))
        (Class|GameplayStatics|CreatePlayer -1)
        (bind _returnvalue (Game|SpawnActorfromClass "/Game/Blueprints/BP_InputReceiver.BP_InputReceiver_C" (Transformation|GetActorTransform (Utilities|Array|Get(acopy) (Variables|Default|GetPlayerStartArray) (LocalVariables|GetIndex))) "Undefined" 0 (LocalVariables|GetIndex) 0))
        (Utilities|Array|AddUnique (Variables|Default|GetPlayerInputReceiverArray) _returnvalue)
        (Pawn|Possess (Game|GetPlayerController (LocalVariables|GetIndex)) _returnvalue)
        (Utilities|Array|AddUnique (Variables|Default|GetPlayerControllerArray) (Game|GetPlayerController (LocalVariables|GetIndex)))))))

(fn NametoInt
  (params (PlayerStart :type Player%20Start%20Object%20Reference))
  (return (Math|Conversions|ToInteger(Byte) (Utilities|String|ToString(Name) (Variables|/Script/Engine.PlayerStart|GetPlayerStartTag PlayerStart)))))

(fn DisplayCharacterSelect
  (params (CurrentPlayerIndex :type Integer))
  (bind _characterselect (Default|AddCharacterSelect (Variables|Default|GetMenuWidjetRed) CurrentPlayerIndex))
  (Variables|/Game/Blueprints/BP_InputReceiver.BP_InputReceiver_C|SetCharacterMenuRef (Utilities|Array|Get(acopy) (Variables|Default|GetPlayerInputReceiverArray) CurrentPlayerIndex) _characterselect)
  (return false))

(fn SpawnPlayer
  (params (CurrentPlayerIndex :type Integer) (CharacterChoice :type Integer) (InputReceiver :type BP%20Input%20Receiver%20Object%20Reference))
  (bind _returnvalue (Game|SpawnActorfromClass "/Game/ThirdPersonBP/Blueprints/ThirdPersonCharacter.ThirdPersonCharacter_C" (Transformation|GetActorTransform InputReceiver) "Undefined" (Game|GetPlayerController CharacterChoice) 0))
  (Pawn|Possess (Game|GetPlayerController CurrentPlayerIndex) _returnvalue)
  (return false))